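; Default_Hud is the shooter's HUD Blueprint, which creates the on-screen W_HUD widget and relays weapon events to it.
; On BeginPlay it creates the widget, adds it to the viewport and keeps a reference.
; OnWeaponChanged and OnWeaponFired check that reference is valid, then pass the weapon to the widget's SetCurrentWeapon and HandleWeaponFired functions.
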(event EventBeginPlay
  (bind _returnvalue (UserInterface|CreateWidget "/Game/UShooter/UI/W_HUD.W_HUD_C"))
  (UserInterface|Viewport|AddtoViewport _returnvalue 0)
  (Variables|Default|SetHUD%20Widget _returnvalue))

(event Collision|EventActorBeginOverlap
  (params (OtherActor :type Actor%20Object%20Reference)))

(event EventOnWeaponFired
  (params (Weapon :type Shooter%20Weapon%20Component%20Object%20Reference))
  (bind _hud_widget (Variables|Default|GetHUD%20Widget))
  (Utilities|IsValid _hud_widget
    (:Is%20Valid
      (Default|HandleWeaponFired _hud_widget Weapon))))

(event EventOnWeaponChanged
  (params (Weapon :type Shooter%20Weapon%20Component%20Object%20Reference))
  (bind _hud_widget (Variables|Default|GetHUD%20Widget))
  (Utilities|IsValid _hud_widget
    (:Is%20Valid
      (Default|SetCurrentWeapon _hud_widget Weapon))))

(event EventTick
  (params (DeltaSeconds :type Float%20%28single-precision%29)))

(fn ConstructionScript)